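; Blueprint function library of mission scripting helpers, covering objectives, VO reminders, screen fades, sequences, loot lookup and assorted math and actor utilities.
; Difficulty helpers pick random floats, ints and weighted bools from per-difficulty inputs and a random stream.
; Metadata helpers take tags and a random stream holder to return bool or int values.
; All function bodies here are empty, returning only defaults or nothing.
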(fn `BitmaskHasValue`
  (params (Bitmask :type Integer) (EnumValue :type Byte))
  (returns (HasValue :type Boolean))
  (return false))

(fn `BreakEscapeVanStopPrefab`
  (params (EscapeVanStop :type "Actor Object Reference"))
  (returns (IsValid :type Boolean) (TrafficPath :type "IGS_TrafficPathComponent Object Reference") (VehicleSpawner :type "IGS_VehicleSpawner Object Reference") (DestinationPoint :type "IGS_VehicleDestinationPoint Object Reference"))
  (locals (Local_TrafficPath :type "IGS_TrafficPathComponent Object Reference") (Local_DestinationPoint :type "IGS_VehicleDestinationPoint Object Reference") (Local_VehicleSpawner :type "IGS_VehicleSpawner Object Reference"))
  (return false "" "" ""))

(fn `Check_isActorOrComponent`
  (params (Object_Ref :type "Object Object Reference"))
  (returns (Component_Ref :type "SceneComponent Object Reference") (isCorrectObject :type Boolean))
  (return "" false))

(fn `Difference (​float)`
  (params (A :type "Object Object Reference") (B :type "Object Object Reference"))
  (returns (ReturnValue :type "Object Object Reference"))
  (return "0.0"))

(fn `Fade In Game`
  (params (FadeTime :type "Object Object Reference"))
  (return))

(fn `FadeInForController`
  (params (inFadeTime :type "Object Object Reference") (InController :type "PlayerController Object Reference"))
  (return))

(fn `FadeOutForController`
  (params (inFadeTime :type "Object Object Reference") (InController :type "Controller Object Reference"))
  (return))

(fn `FadeOutGame`
  (params (FadeTime :type "Object Object Reference"))
  (return))

(fn `GetActorLevelName`
  (params (Actor :type "Actor Object Reference"))
  (returns (Level :type "Object Object Reference"))
  (return ""))

(fn `GetBoolMetaData`
  (params (MetaData_Map :type "Map of GameplayTag Object Reference to Integer") (MetaTag :type "GameplayTag Object Reference") (RandomStreamHolder :type "IGS_RandomStreamHolder Object Reference"))
  (returns (MetaValue :type Boolean) (MetaTagFound :type Boolean))
  (return false false))

(fn `GetIntMetaData`
  (params (MetaData_Map :type "Map of GameplayTag Object Reference to Integer") (MetaTag :type "GameplayTag Object Reference") (Range :type "META_Interval Object Reference") (RandomStreamHolder :type "IGS_RandomStreamHolder Object Reference"))
  (returns (MetaValue :type Integer) (MetaTagFound :type Boolean))
  (return 0 false))

(fn `GetLootTypeAndValueFromID`
  (params (ObjectLootID :type "Object Object Reference") (inWCO :type "Actor Object Reference"))
  (returns (LootTypeTag :type "GameplayTagContainer Object Reference") (LootValue :type Integer))
  (return "" 0))

(fn `GetMissionDifficulty`
  (params (`World Context Object` :type "Object Object Reference"))
  (returns (Difficulty :type "EIGS_ScenarioDifficulty Enum"))
  (return "SD_Unknown"))

(fn `GetSortedByDistanceTo`
  (params (Target :type "Actor Object Reference") (Actors :type "Array of Actor Object Reference (by ref)") (Descending :type Boolean))
  (returns (SortedActors :type "Array of Actor Object Reference"))
  (locals (Local_NewIndices :type "Array of Integer") (Local_SortedArray :type "Array of Actor Object Reference") (Local_Descending :type Boolean) (Local_Distances :type "Array of Object Object Reference"))
  (return))

(fn `Handle_Bool_MetaData`
  (params (EditorCustomValue :type Integer) (MetaTag :type "GameplayTag Object Reference") (RandomStreamHolder :type "IGS_RandomStreamHolder Object Reference") (WorldContextObject :type "Object Object Reference"))
  (returns (`Bool Meta Value` :type Boolean))
  (return false))

(fn `Handle_Int_MetaData`
  (params (EditorCustomValue :type Integer) (MetaTag :type "GameplayTag Object Reference") (Range :type "META_Interval Object Reference") (RandomStreamHolder :type "IGS_RandomStreamHolder Object Reference") (WorldContextObject :type "Object Object Reference"))
  (returns (`Int Meta Value` :type Integer))
  (return 0))

(fn `HideSession`
  (return))

(fn `Infinity (​float)`
  (returns (PositiveInfinity :type "Object Object Reference") (NegativeInfinity :type "Object Object Reference"))
  (return "0.0" "0.0"))

(fn `NumericLimits (​int)`
  (returns (MinValue :type Integer) (MaxValue :type Integer))
  (locals (Local_Max :type Integer))
  (return 0 0))

(fn `ObjectiveCompleted`
  (params (ObjectiveComponent :type "IGS_ObjectiveComponent Object Reference"))
  (return))

(fn `ObjectiveDecrease`
  (params (ObjectiveComponent :type "IGS_ObjectiveComponent Object Reference"))
  (return))

(fn `ObjectiveFailed`
  (params (ObjectiveComponent :type "IGS_ObjectiveComponent Object Reference"))
  (return))

(fn `ObjectiveIncrease`
  (params (ObjectiveComponent :type "IGS_ObjectiveComponent Object Reference"))
  (return))

(fn `PlaySequence`
  (params (Sequence :type "LevelSequenceActor Object Reference"))
  (return))

(fn `Random Bool ​with Weight ​by Difficulty`
  (params (GameState :type "IGS_GameStateGame Object Reference") (Easy :type "Object Object Reference") (Medium :type "Object Object Reference") (Hard :type "Object Object Reference") (`Random Stream` :type "RandomStream Object Reference"))
  (returns (ReturnValue :type Boolean))
  (locals (RandomBoolByDifficulty :type Boolean))
  (return false))

(fn `Random Float by Difficulty`
  (params (GameState :type "IGS_GameStateGame Object Reference") (EasyMin :type "Object Object Reference") (EasyMax :type "Object Object Reference") (MedMin :type "Object Object Reference") (MedMax :type "Object Object Reference") (HardMin :type "Object Object Reference") (HardMax :type "Object Object Reference") (`Random Stream` :type "RandomStream Object Reference"))
  (returns (RandomFloatByDifficulty :type "Object Object Reference"))
  (locals (RandomFloatByDiff :type "Object Object Reference"))
  (return "0.0"))

(fn `Random Int by Difficulty`
  (params (GameState :type "IGS_GameStateGame Object Reference") (EasyMin :type Integer) (EasyMax :type Integer) (MedMin :type Integer) (MedMax :type Integer) (HardMin :type Integer) (HardMax :type Integer) (`Random Stream` :type "RandomStream Object Reference"))
  (returns (RandomIntByDifficulty :type Integer))
  (locals (RandomIntByDiff :type Integer))
  (return 0))

(fn `RemoveLoadingFaderScreen`
  (return))

(fn `RoundWithPrecision (​float)`
  (params (A :type "Object Object Reference") (Precision :type Integer))
  (returns (ReturnValue :type "Object Object Reference"))
  (return "0.0"))

(fn `TakeOutWeapon`
  (params (LocalPC :type "Controller Object Reference"))
  (return))

(fn `VO_Reminder_Clear_Dialogue`
  (return))

(fn `VO_Reminder_Set_Multiple_Variants`
  (params (Stealth_Dialogues :type "Array of Object Object Reference (by ref)") (Combat_Dialogues :type "Array of Object Object Reference (by ref)"))
  (return))

(fn `VO_Reminder_Set_Single_Dialogue`
  (params (Stealth_Dialogue :type "Object Object Reference") (Combat_Dialogue :type "Object Object Reference"))
  (return))

(fn `Widget Enum Converter`
  (params (OldEnum :type "/Game/00_Main/Blueprints/Enums/E_WaypointTypes Enum" :default "NewEnumerator0"))
  (returns (NewEnum :type "EIGS_WorldWidgetType Enum"))
  (return "Widget_Hidden"))