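; Escape vehicle component for ending a mission through a trigger that players gather in.
; Its interface covers server trigger setup, enabling and disabling, and replicated counts of players inside versus alive, with hooks for joins, deaths and disconnects.
; Further events and functions cover the ending: hiding characters, making players and bots unkillable, fading to black, swapping camera and spawning escape paperdolls.
; All bodies here are empty stubs.
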(event `HideCharacters`)

(event `UpdatePlayersUI`)

(event `HidePlayersInEndMissionTrigger`)

(event `self.ReceiveBeginPlay`)

(event `SetPaperdoll`
  (params (paperdoll :type "PaperDollAbstract Object Reference") (Animation :type "AnimMontage Object Reference")))

(event `MultiFadeBlack`)

(event `UpdatePlayersInEscapeTrigger`)

(event `PlayerDisconnected`
  (params (PlayerController :type "PlayerController Object Reference")))

(event `HandlePlayerDeath`
  (params (CurrentHealth :type "Object Object Reference") (CurrentShield :type "Object Object Reference") (HealthChange :type "Object Object Reference") (ShieldChange :type "Object Object Reference") (HitInfo :type "IGS_HitInfo Object Reference (by ref)")))

(event `DisableEndMissionTrigger`)

(event `Server_SetupEndMissionTrigger`
  (params (inTrigger :type "/Game/00_Main/Blueprints/Triggers/BP_EndMission_Trigger Object Reference (by ref)") (InEndMissionTriggerLocation :type "Vector Object Reference") (InHidePlayersAtEndMission :type Boolean)))

(event `PlayersInEndMissionChanged`
  (params (NumPlayersInside :type Integer) (NumAlivePlayersTotal :type Integer)))

(event `VehicleEndMission`)

(event `EnableEndMissionTrigger`)

(event `OnPlayerJoined`
  (params (inGameCharacter :type "IGS_GameCharacterFramework Object Reference")))

(event `SpawnEscapePaperdoll`
  (params (VehcileBase :type "SkeletalMeshComponent Object Reference") (Animation :type "AnimMontage Object Reference") (SpawnTransform :type "Transform Object Reference") (CharacterID :type "EIGS_CharacterID Enum" :default "Char_Unknown") (isMaxedLeveld :type Boolean) (CharacterVariant :type Integer) (Character :type "IGS_GameCharacterFramework Object Reference")))

(event `VehicleEndMissionServer`)

(fn `HandlePlayersDeath`
  (locals (LocalTotalPlayers :type Integer))
  (return))

(fn `OnRep_Num Alive Players Total`
  (return))

(fn `OnRep_Num Players Inside`
  (return))

(fn `SetAllBotsUnkillable`
  (return))

(fn `SetAllPlayersUnkillable`
  (return))

(fn `SetupEndMissionTrigger`
  (params (inTrigger :type "/Game/00_Main/Blueprints/Triggers/BP_EndMission_Trigger Object Reference (by ref)") (InEndMissionPlayerLocation :type "Vector Object Reference") (InHidePlayersAtEndMission :type Boolean) (EndMIssionSequence :type "Object Object Reference (by ref)"))
  (return))

(fn `Swapcamera`
  (params (CameraSetup :type "CineCameraComponent Object Reference") (SpawnTransform :type "Transform Object Reference"))
  (returns (ReturnValue :type "CineCameraActor Object Reference"))
  (locals (CameraComponent :type "CineCameraComponent Object Reference"))
  (return ""))