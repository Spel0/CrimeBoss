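; BP_LootManagerComponent is a loot manager component whose function names cover choosing and spawning allowed special and simple loot for a mission.
; It declares functions for gathering special spawners, checking mission spawner counts, setting quickplay special loot, converting specific loot and fetching debug loot lists.
; All are empty stubs: BeginPlay does nothing, both boolean functions return false, and the others return without logic.
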(event `self.ReceiveBeginPlay`)

(fn `GetAllowedLoot`
  (returns (AllowedLoot :type "Array of GameplayTag Object Reference"))
  (return))

(fn `GetAllSpecialSpawners`
  (return))

(fn `GetDebugAllowedLoot`
  (returns (AllowedLoot :type "Array of GameplayTag Object Reference"))
  (return))

(fn `GetDebugSimpleAllowedLoot`
  (returns (AllowedLoot :type "Array of GameplayTag Object Reference"))
  (return))

(fn `GetDebugSpecialAllowedLoot`
  (returns (AllowedLoot :type "Array of GameplayTag Object Reference"))
  (locals (Local_AllowedLoot :type "GameplayTag Object Reference") (Local_SpecialLoot :type "IGS_SpecialLoot Object Reference"))
  (return))

(fn `MissionHasEnoughSpecialSpawners`
  (returns (ReturnValue :type Boolean))
  (return false))

(fn `SetQuickplaySpecialLoot`
  (returns (HasSpecialLoot :type Boolean))
  (locals (LocalSpecialLoot :type "IGS_SpecialLoot Object Reference"))
  (return false))

(fn `SpawnSimpleAllowedLoot`
  (locals (Local_Spawner :type "/Game/00_Main/Blueprints/Gameplay/Spawners/BP_SPAWNER_SpecialLootCollection Object Reference"))
  (return))

(fn `SpawnSpecialAllowedLoot`
  (locals (Local_Spawner :type "/Game/00_Main/Blueprints/Gameplay/Spawners/BP_SPAWNER_SpecialLootCollection Object Reference") (CurrentLootTypeIndex :type Integer))
  (return))

(fn `SpecialLootToAllowedLoot`
  (params (SpecificLoot :type "Array of IGS_SpecificSpecialLoot Object Reference (by ref)"))
  (returns (AllowedLoot :type "Array of GameplayTag Object Reference"))
  (locals (Local_AllowedLoot :type "Array of GameplayTag Object Reference"))
  (return))