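; Multiplayer Game Instance that declares game-wide control of online sessions, level travel and mission state.
; Session events cover hosting, joining, invites, visibility and lobby/in-progress state, alongside privilege checks with cached results.
; Further hooks cover level-load and fade transitions, mission chaining, save/load, and modals for network loss, controller disconnect and quitting.
; All events and functions here are empty stubs, with async success/failure callbacks unwired.
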(event `OnSuccess_A7B85191454BACD2D3362E89D16763CF`
  (params (QueriedPrivilege :type "EBPUserPrivileges Enum" :default "CanPlay") (HadPrivilege :type Boolean)))

(event `HostFromLobby`
  (params (PlayerController :type "PlayerController Object Reference") (`Server Settings` :type "/Game/00_Main/Core/ServerSettings Object Reference") (OptionString :type "Object Object Reference")))

(event `OnSuccess_D54872984F7DA9FB56648F8B3B1C6341`)

(event `Quit To Menu`
  (params (PlayerController :type "PlayerController Object Reference") (ForceResult :type "ECommonMissionResult Enum" :default "Res_UNKNOWN")))

(event `OnFailure_222BD362473730B45A8388B49FE8C74B`)

(event `SetCurrentMission`
  (params (CurrentMissione :type "/Game/00_Main/Maps/Menu/Struct_CurrentMission Object Reference")))

(event `OnFailure_1BC9FAFC42B8981F3B2F788C23CC7537`
  (params (Results :type "Array of BlueprintSessionResult Object Reference (by ref)")))

(event `LevelTransitionStateChanged`
  (params (inCurrentState :type "EIGS_LevelTransitionType Enum" :default "LT_Unknown") (inPreviousState :type "EIGS_LevelTransitionType Enum" :default "LT_Unknown")))

(event `OnFailure_E3D7BAB045E1C5ED4FC80AAE54C5C51E`)

(event `OnCancelled_EBA428C14BD8639EFE0052BA11E2562C`)

(event `HandlePingThrowBagRebind`)

(event `LevelLoadAttemptSuccess_61644BB2414C81B5A90363ACA60D3C4C`)

(event `FadeOutGame`
  (params (FadeTime :type "Object Object Reference")))

(event `LevelLoadAttemptSuccess_FF16108C499286D4EF8E1DBA30F2C3F2`)

(event `OnControllerInputEstablished`)

(event `LevelLoadAttemptFailure_EB6068B244DAFB857CA096B46327291D`)

(event `ChangeSystemSessionVisibility`
  (params (bShouldAdvertise :type Boolean)))

(event `OnSuccess_222BD362473730B45A8388B49FE8C74B`)

(event `self.OnConnectionStatusChangedEvent`
  (params (InStatus :type "EIGS_PlatformServerConnectionStatus Enum" :default "Unknown")))

(event `OnSuccess_A7B85191454BACD2D3362E89E92516E7`
  (params (QueriedPrivilege :type "EBPUserPrivileges Enum" :default "CanPlay") (HadPrivilege :type Boolean)))

(event `LevelLoadStarted_3832DFCD45BE5659FF33B4A620A9C9CF`)

(event `self.OnSessionInviteAccepted`
  (params (LocalPlayerNum :type Integer) (PersonInvited :type "BPUniqueNetId Structure") (SessionToJoin :type "BlueprintSessionResult Structure (by ref)")))

(event `OnSuccess_DECE2D8A4A013E2B956A3A85B92E2841`)

(event `LevelLoadAttemptSuccess_B202906D4AFB4B56A3290AB4D8644699`)

(event `OnTransitionFinished_491CB16D44A93111A54807AB5078C789`)

(event `DestroyFadeScreen`)

(event `OnFailure_A7B85191454BACD2D3362E891DAD7020`)

(event `LevelLoadFinished`
  (params (CurrentState :type "EIGS_LevelTransitionType Enum" :default "LT_Unknown") (PreviousState :type "EIGS_LevelTransitionType Enum" :default "LT_Unknown")))

(event `OnTransitionFinished_9063FB7148175EBE38109BB09D9EF029`)

(event `OnFailure_DF3C6F2142E1223A96C387BEE2CEA25D`)

(event `OnExtraOption_9B0C4C7C4CA72F008BAF5B8D9B1A7622`)

(event `AllowInvites`)

(event `LevelLoadStarted_61644BB2414C81B5A90363ACA60D3C4C`)

(event `self.QuitToLobby`
  (params (inWCO :type "Object Object Reference") (inMissionResult :type "ECommonMissionResult Enum" :default "Res_UNKNOWN")))

(event `OnFailure_11A78EE74CC69B40330006A8F1BE95E3`)

(event `OnLevelLoadStarted`
  (params (LevelName :type "Object Object Reference") (ServerTravel :type Boolean)))

(event `LevelLoadAttemptSuccess_E42FF7734EF52E95412E7287F73B8335`)

(event `ChangeUserSessionVisibility`
  (params (bShouldAdvertise :type Boolean)))

(event `OnExtraOption_162A4965420E22973A001A9DE06E2F5E`)

(event `UpdateMissionID`
  (params (inID :type "Guid Object Reference")))

(event `LevelLoadAttemptFailure_D6A3B7D14EF552C307619E97571D3026`)

(event `OnFailure_57CA8D8E4459C56A98B9BEAB8936DDEE`)

(event `LevelLoadAttemptSuccess_3D47473B43E62CEFFDECDFB22A596FC7`)

(event `LevelLoadStarted_B202906D4AFB4B56A3290AB4D8644699`)

(event `LevelLoadAttemptSuccess_0102BA5B405DC9FC9CCA3A93D88ABE33`)

(event `self.OnApplicationHasReactivated`)

(event `LevelLoadAttemptFailure_FF16108C499286D4EF8E1DBA30F2C3F2`)

(event `SetSessionStateToInProgress`)

(event `OnFailure_CE7F99DB42FA8F632F8EE9BD1FE1C0A9`)

(event `HideSessionInternal`)

(event `OnFailure_978320DD4FAA0CDFDBF76FBB999EC785`)

(event `LevelLoadStarted_0CB48DDD4558BBACC5413CBC8A94C0DD`)

(event `RequestOpenConnectionLostModalScreen`
  (params (inReason :type "Object Object Reference") (reloadToMainMenu :type Boolean)))

(event `OnFailure_A7B85191454BACD2D3362E8934830072`)

(event `ServerTravelToMap`
  (params (inLevelName :type "Object Object Reference")))

(event `OnFailure_6A23D45D4A4F79B29E1F388319F34D7D`)

(event `self.HandleNetworkError`
  (params (FailureType :type "ENetworkFailure Enum" :default "NetDriverAlreadyExists") (bIsServer :type Boolean)))

(event `LevelLoadStarted_E42FF7734EF52E95412E7287F73B8335`)

(event `ReturnFromMission`)

(event `OnSuccess_1BC9FAFC42B8981F3B2F788C23CC7537`
  (params (Results :type "Array of BlueprintSessionResult Object Reference (by ref)")))

(event `self.OnWindowStateChanged`
  (params (inState :type Boolean)))

(event `OnTransitionFinished_C27C6CF64C8F32C5A74581AA3B7DFCF7`)

(event `OnExtraOption_EBA428C14BD8639EFE0052BA11E2562C`)

(event `LevelLoadStarted_3D47473B43E62CEFFDECDFB22A596FC7`)

(event `LevelLoadAttemptFailure_0CB48DDD4558BBACC5413CBC8A94C0DD`)

(event `LevelLoadStarted_0102BA5B405DC9FC9CCA3A93D88ABE33`)

(event `self.JoinSessionFailed`
  (params (Reason :type "EIGS_SessionJoinFailureReason Enum" :default "FR_SessionIsFull")))

(event `LevelLoadAttemptSuccess_EB6068B244DAFB857CA096B46327291D`)

(event `HideSession`)

(event `OnFailure_DE1B07AD456FE54911107F8D0B92C92F`)

(event `CreateBaseSession`)

(event `OnFailure_BBF663D140791F358CE7D5A58D51545C`)

(event `LevelLoadAttemptFailure_3832DFCD45BE5659FF33B4A620A9C9CF`)

(event `StartedPlaying`)

(event `OnFailure_A7B85191454BACD2D3362E89D16763CF`)

(event `Restart Level`)

(event `OnFailure_D54872984F7DA9FB56648F8B3B1C6341`)

(event `Join Server`
  (params (PlayerController :type "PlayerController Object Reference") (SearchResult :type "BlueprintSessionResult Object Reference (by ref)")))

(event `OnTransitionFinished_F490BA734B1F624A0080FA8BD54B6277`)

(event `DestroyBlackScreen`)

(event `OnSuccess_A7B85191454BACD2D3362E891DAD7020`
  (params (QueriedPrivilege :type "EBPUserPrivileges Enum" :default "CanPlay") (HadPrivilege :type Boolean)))

(event `ChangeSystemSessionVisibilityWithoutUpdate`
  (params (bShouldAdvertise :type Boolean)))

(event `OnTransitionFinished_3C56AEFE49F331ADDB0646AF04983A8D`)

(event `OnSuccess_DF3C6F2142E1223A96C387BEE2CEA25D`)

(event `OnConfirmed_9B0C4C7C4CA72F008BAF5B8D9B1A7622`)

(event `SessionCreationFinished_Event`
  (params (Successful :type Boolean)))

(event `LevelLoadAttemptFailure_61644BB2414C81B5A90363ACA60D3C4C`)

(event `FadeInGame`
  (params (FadeTime :type "Object Object Reference")))

(event `OnSuccess_11A78EE74CC69B40330006A8F1BE95E3`)

(event `OnCurrentControllerDisconnected`)

(event `LevelLoadStarted_EB6068B244DAFB857CA096B46327291D`)

(event `UpdateSessionVisibilityInternal`)

(event `OnConfirmed_162A4965420E22973A001A9DE06E2F5E`)

(event `SavePreviousMissionID`
  (params (PreviousMissionID :type "Guid Object Reference")))

(event `OnFailure_A7B85191454BACD2D3362E89E92516E7`)

(event `LevelLoadAttemptSuccess_D6A3B7D14EF552C307619E97571D3026`)

(event `OnSuccess_57CA8D8E4459C56A98B9BEAB8936DDEE`)

(event `OnFailure_DECE2D8A4A013E2B956A3A85B92E2841`)

(event `LevelLoadAttemptFailure_B202906D4AFB4B56A3290AB4D8644699`)

(event `OnTransitionFinished_C54B4291433AE7B0AC0AA49EB044762B`)

(event `CheckPrivilege`
  (params (Privilege :type "EBPUserPrivileges Enum" :default "CanPlay")))

(event `OnSuccess_E3D7BAB045E1C5ED4FC80AAE54C5C51E`)

(event `SetSessionStateToInLobby`)

(event `OnSuccess_CE7F99DB42FA8F632F8EE9BD1FE1C0A9`)

(event `OnUpdateSessionStatus`)

(event `OnSuccess_978320DD4FAA0CDFDBF76FBB999EC785`)

(event `OnCancelled_9B0C4C7C4CA72F008BAF5B8D9B1A7622`)

(event `RefreshSessions`)

(event `OnSuccess_A7B85191454BACD2D3362E8934830072`
  (params (QueriedPrivilege :type "EBPUserPrivileges Enum" :default "CanPlay") (HadPrivilege :type Boolean)))

(event `CreateBlackScreen`)

(event `OnSuccess_6A23D45D4A4F79B29E1F388319F34D7D`)

(event `self.ReceiveInit`)

(event `LevelLoadAttemptFailure_E42FF7734EF52E95412E7287F73B8335`)

(event `SetChainMission`
  (params (IsActive :type Boolean)))

(event `OnCancelled_162A4965420E22973A001A9DE06E2F5E`)

(event `self.OnApplicationHasEnteredForeground`)

(event `LevelLoadStarted_D6A3B7D14EF552C307619E97571D3026`)

(event `OnConfirmed_EBA428C14BD8639EFE0052BA11E2562C`)

(event `LevelLoadAttemptFailure_3D47473B43E62CEFFDECDFB22A596FC7`)

(event `LevelLoadAttemptSuccess_0CB48DDD4558BBACC5413CBC8A94C0DD`)

(event `LevelLoadAttemptFailure_0102BA5B405DC9FC9CCA3A93D88ABE33`)

(event `SavePreviousSessionID`
  (params (PreviousSessionID :type "Object Object Reference")))

(event `LevelLoadStarted_FF16108C499286D4EF8E1DBA30F2C3F2`)

(event `UpdateSessionVisibility`)

(event `OnSuccess_DE1B07AD456FE54911107F8D0B92C92F`)

(event `AltF4ModalRequested`)

(event `OnSuccess_BBF663D140791F358CE7D5A58D51545C`)

(event `LevelLoadAttemptSuccess_3832DFCD45BE5659FF33B4A620A9C9CF`)

(event `RequestOpenControllerDisconnectedModalScreen`)

(fn `GetCachedPrivilege`
  (params (Privilege :type "EBPUserPrivileges Enum" :default "CanPlay"))
  (returns (HasPrivilegeCache :type Boolean))
  (return false))

(fn `GetGlobalShouldAdvertise`
  (returns (`Return Value` :type Boolean))
  (return false))

(fn `GetMissionData`
  (returns (MissionData :type "/Game/00_Main/Maps/Menu/UMissionData Object Reference"))
  (return ""))

(fn `GetNetworkErrorMessage`
  (params (NetworkFailure :type "ENetworkFailure Enum" :default "NetDriverAlreadyExists"))
  (returns (ErrorMessage :type "Object Object Reference"))
  (locals (LocalErrorText :type "Object Object Reference"))
  (return ""))

(fn `GetPreviousMissionID`
  (returns (PreviousMissionID :type "Guid Object Reference"))
  (return ""))

(fn `GetPreviousSessionID`
  (returns (PreviousSession :type "Object Object Reference"))
  (return ""))

(fn `GetUserShouldAdvertise`
  (returns (outAdvertise :type Boolean))
  (return false))

(fn `Is in Online Mode`
  (returns (InOnlineMode :type Boolean))
  (return false))

(fn `IsChainMission`
  (returns (IsChainMission :type Boolean))
  (return false))

(fn `IsProcessingInvite`
  (returns (Result :type Boolean))
  (return false))

(fn `IsTextChatAllowed`
  (returns (ReturnValue :type Boolean))
  (return false))

(fn `JIPAllowed`
  (params (Session :type "BlueprintSessionResult Object Reference"))
  (returns (Allowed :type Boolean))
  (return false))

(fn `LoadGameInstanceData`
  (return))

(fn `NotifyPrivilegeCheckResult`
  (params (Privilege :type "EBPUserPrivileges Enum" :default "CanPlay") (HasPrivilege :type Boolean))
  (returns (PrivilegeChanged :type Boolean))
  (return false))

(fn `OnConnectionLostConfirmed`
  (params (ReloadToMenuAfterModal :type Boolean))
  (return))

(fn `OnWindowCloseRequested`
  (returns (ReturnValue :type Boolean))
  (return false))

(fn `QuitLobby`
  (return))

(fn `SaveGameInstanceData`
  (params (AccountSaveGame :type "IGS_PaybackSaveGameAccount Object Reference"))
  (return))