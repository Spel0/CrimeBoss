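; BP_GameState is the game state Blueprint for a heist game, declaring match-wide mission flow from player spawn through alarm, escape and mission end.
; Events cover all heisters downed, boss death, end-mission countdowns, restart and server travel, plus bindings to suspicion alarms and text chat.
; Functions handle exit areas, bot heister numbers, HUD messages and manager access, with RepNotifies for loot bar, bonus objectives and mission ID.
; All graph bodies shown are empty stubs.
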(event `Multicast_AddHUDMessage`
  (params (InText :type "Object Object Reference") (inDuration :type "Object Object Reference") (inCountdown :type Integer)))

(event `Alarmed`
  (params (inAlarmReason :type "EIGS_AlarmReason Enum" :default "Alarm_UNKNOWN")))

(event `HandleLootBarGoalValue`)

(event `BndEvt__TextChatManager_K2Node_ComponentBoundEvent_0_BF_TextMessageSentSignature__DelegateSignature`
  (params (inMessage :type "Object Object Reference") (inPlayerName :type "Object Object Reference") (inHeisterNum :type Integer)))

(event `self.PostInit`)

(event `RemoveBotInvulnerability`)

(event `self.OnAllDiedOrDowned`)

(event `self.FinishEndMissionNoResultScreen`)

(event `self.OnPrepareRestart`)

(event `self.ReceiveEndPlay`
  (params (EndPlayReason :type "EEndPlayReason Enum" :default "Destroyed")))

(event `self.OnServerTravel`)

(event `self.OnMatchHasEnded`)

(event `Escape`)

(event `self.OnStartedPlayingMatch`)

(event `self.OnBossDied`
  (params (inCharacterID :type "EIGS_CharacterID Enum" :default "Char_Unknown")))

(event `self.StartEndMission`
  (params (inMissionResult :type "ECommonMissionResult Enum" :default "Res_UNKNOWN")))

(event `FinalDialogueFinished`)

(event `BndEvt__SuspicionManager_K2Node_ComponentBoundEvent_3_BF_AlarmedSignature__DelegateSignature`
  (params (AlarmReason :type "EIGS_AlarmReason Enum" :default "Alarm_UNKNOWN")))

(event `HandleLootBar`)

(event `self.HandleEndMissionCountdownPreCompleted`)

(event `self.ReceiveBeginPlay`)

(event `ExitArea`)

(event `self.HandleEndMissionCountdownCompleted`)

(event `self.OnPlayersSpawned`)

(event `ForceKillAllHeisters`
  (params (DownState :type Boolean)))

(event `self.FinishEndMission`)

(fn `ActivateExitAreas`
  (return))

(fn `AddHUDMessage`
  (params (InText :type "Object Object Reference") (inDuration :type "Object Object Reference") (inCountdown :type Integer))
  (return))

(fn `Get Horde Mode Manager`
  (returns (HordeModeManager :type "/Game/00_Main/Maps/SmallHits/HOR_HordeMode/BP_HordeModeManager Object Reference"))
  (return ""))

(fn `GetHeisterNumberFromBotBP`
  (params (inBot :type "Controller Object Reference"))
  (returns (ReturnValue :type Integer))
  (return 0))

(fn `GetLootManager`
  (returns (ReturnValue :type "IGS_LootManager Object Reference"))
  (return null))

(fn `HideLootBar`
  (return))

(fn `OnRep_BonusObjectiveManager`
  (return))

(fn `OnRep_bShowLootBar`
  (return))

(fn `OnRep_GoalValue`
  (return))

(fn `OnRep_MissionUniqueID`
  (return))

(fn `SetBonusObjectiveManager`
  (return))

(fn `SetHeisterNumberForBotBP`
  (params (inBot :type "Controller Object Reference") (inHeisterID :type Integer :default 0))
  (returns (ReturnValue :type Integer))
  (return 0))

(fn `SetLootBarGoalValue`
  (params (InValue :type "Object Object Reference"))
  (return))

(fn `ShowLootBar`
  (return))