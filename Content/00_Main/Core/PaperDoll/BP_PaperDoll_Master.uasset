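; BP_PaperDoll_Master is, by its name, the master Blueprint for paperdoll characters, declaring hooks for animation, appearance and dialogue.
; Its events cover animation setup with random start, montage play and stop, async loading, and dialogue line start and finish.
; Its functions cover morphs, custom stencil, lighting channels including props, facials, speaker lookup and internal voice playback.
; Every event and function body here is empty or returns a default, so no behavior is implemented.
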(event `self.ReceiveBeginPlay`)

(event `OnDialogueFinished`)

(event `StopMontageOnPaperdoll`)

(event `OnInterrupted_92CF8F5B4E52AE788ABB41AE9380DF51`
  (params (NotifyName :type "Object Object Reference")))

(event `OnLoaded_178A48AF4808B130754A32B3D15889BB`
  (params (Loaded :type "Object Object Reference")))

(event `PlayMontageOnPaperdoll`
  (params (`Anim Montage` :type "AnimMontage Object Reference")))

(event `InitAnimations`)

(event `OnNotifyBegin_92CF8F5B4E52AE788ABB41AE9380DF51`
  (params (NotifyName :type "Object Object Reference")))

(event `OnCompleted_92CF8F5B4E52AE788ABB41AE9380DF51`
  (params (NotifyName :type "Object Object Reference")))

(event `OnDialogueLineStarted`
  (params (LineID :type "Object Object Reference") (DialogueSlot :type "EIGS_MetaDialogueCharacterSlot Enum" :default "None") (LineOrderID :type Integer) (LinesCount :type Integer) (inVoiceLenght :type "Object Object Reference")))

(event `SetRandomAnimationStart`
  (params (Min :type "Object Object Reference") (Max :type "Object Object Reference") (RandomizeAnimationPlayStart :type Boolean)))

(event `OnNotifyEnd_92CF8F5B4E52AE788ABB41AE9380DF51`
  (params (NotifyName :type "Object Object Reference")))

(event `OnBlendOut_92CF8F5B4E52AE788ABB41AE9380DF51`
  (params (NotifyName :type "Object Object Reference")))

(fn `GetThisPaperDollSpeaker`
  (returns (outSpeaker :type "EIGS_MetaDialogueSpeaker Enum"))
  (return "None"))

(fn `GetVoiceProgressInternal`
  (params (inGroupID :type Integer :default 0))
  (returns (ReturnValue :type "Float (double-precision)"))
  (return 0.0))

(fn `IsPlayingVoiceInternal`
  (params (inGroupID :type Integer :default 0) (inCharacter :type "IGS_DialogueGroupCharacterHolder Structure (by ref)"))
  (returns (ReturnValue :type Boolean))
  (return false))

(fn `PlayDialogueVoiceInternal`
  (params (inVariationData :type "IGS_PlayVariationData Structure (by ref)"))
  (return))

(fn `Set Character Morphs`
  (params (Character_Morphs :type "/Game/00_Main/Core/PaperDoll/ST_PaperDoll_Morphs Object Reference"))
  (locals (BodyComp :type "SkeletalMeshComponentBudgeted Object Reference") (HeadComp :type "SkeletalMeshComponentBudgeted Object Reference"))
  (return))

(fn `SetCustomStencil`
  (params (Stencil :type Integer))
  (return))

(fn `SetLightingChannels`
  (return))

(fn `SetVoiceVoice2DModeEnabledInternal`
  (params (inState :type Boolean :default false))
  (return))

(fn `StopDialogueVoiceInternal`
  (params (inVariationData :type "IGS_PlayVariationData Structure (by ref)"))
  (return))

(fn `Turn Off Facials`
  (return))

(fn `UpdatePaperdollLightChannelsForProps`
  (return))

(fn `UserConstructionScript`
  (return))