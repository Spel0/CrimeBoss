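; BP_ScriptManagerBase is the base mission script manager for what appears to be a heist game with alarms, police assaults and escape vans.
; Its events cover mission start and end, alarm and assault phases, star-based wave manager setup, SWAT tiers, player deaths, blackscreen dialogue and voice-over reminders.
; SCMEvent events look like hooks for mission-specific scripts.
; All events and functions here are empty or return defaults, so only the interface is visible.
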(event `Setup_WaveManagerCustomTags`
  (params (WaveManagerTags :type "Array of GameplayTagContainer Object Reference (by ref)")))

(event `AssembleScriptBase`)

(event `SCMEvent_OnLastPlayerOrBotAlive`
  (params (AlivePlayerOrBot :type "IGS_GameCharacterFramework Object Reference")))

(event `self.ReceiveEndPlay`
  (params (EndPlayReason :type "EEndPlayReason Enum" :default "Destroyed")))

(event `DialogueLineFinished_447BA1524613421CE358B482FA6FBBB9`
  (params (LineIndex :type Integer)))

(event `SCM_Base_StrikeAdded`
  (params (inStrikeCount :type Integer) (inStrikeIncrease :type Integer) (inBlameText :type "Object Object Reference (by ref)")))

(event `DialogueStarted_80BA75504AD858512EDC068FCB7C460B`
  (params (LineIndex :type Integer)))

(event `SCM_Base_PhaseChanged`
  (params (inPressurePhase :type "EIGS_PressurePhase Enum" :default "PP_Unknown")))

(event `DialogueLineFinished_007EBB0340ADB5772A956A9D2C2A325C`
  (params (LineIndex :type Integer)))

(event `Setup_CustomStars`
  (params (Amount :type Integer)))

(event `DialogueFinished_E646BE0948CB57B3E0F0CE9BEE89CA41`
  (params (LineIndex :type Integer)))

(event `SCM_Base_ControlStarted`)

(event `Leave_110789DA42D5AE8606F227A148892C07`
  (params (Character :type "IGS_GameCharacterFramework Object Reference")))

(event `SetupSegment_4Stars`)

(event `DialogueFinished_BF4B34754166F7B85E4D4985665BA794`
  (params (LineIndex :type Integer)))

(event `VO_StopReminder`)

(event `VO_First_SWAT`
  (params (inInstigator :type "IGS_VehicleBase Object Reference")))

(event `DialogueFinished_B5CE670B45EDF888D163B9A9D94FD0B8`
  (params (LineIndex :type Integer)))

(event `SCM_SmallHit_DetectivesArrived`
  (params (inInstigator :type "IGS_VehicleBase Object Reference")))

(event `PlayBlackscreenDialogues`
  (params (BlackscreenIDs :type "Array of Object Object Reference (by ref)") (BlackscreenAudio :type "Array of /Game/00_Main/Blueprints/Enums/S_ScriptManager_AudioDelay Object Reference (by ref)") (InitBlackscreenDelay :type "Object Object Reference") (EndBlackscreenDelay :type "Object Object Reference")))

(event `PlayBlackscreenCharacterDialogues`
  (params (BlackscreenIDs :type "Array of Object Object Reference (by ref)") (DialogueCharacters :type "Map of Integer to /Game/00_Main/Blueprints/Gameplay/Common/struct_ArrayOfActors Object Reference") (BlackscreenAudio :type "Array of /Game/00_Main/Blueprints/Enums/S_ScriptManager_AudioDelay Object Reference (by ref)") (TimeBetweenDialogues :type "Array of Object Object Reference (by ref)") (`End Blackscreen Delay` :type "Object Object Reference") (InitBlackscreenDelay :type "Object Object Reference")))

(event `self.OnManagerReady`
  (params (inReplicatedSeed :type Integer)))

(event `DialogueFinished_007EBB0340ADB5772A956A9D2C2A325C`
  (params (LineIndex :type Integer)))

(event `SCM_Base_GenListener_Heard`
  (params (inActor :type "Actor Object Reference") (inStimulus :type "AIStimulus Object Reference")))

(event `DialogueLineStarted_80BA75504AD858512EDC068FCB7C460B`
  (params (LineIndex :type Integer)))

(event `SCM_Base_SwitchToAssault`
  (params (InstantStorm :type Boolean)))

(event `DialogueFinished_564B97D3460CBFFC602F72A8EE34575F`
  (params (LineIndex :type Integer)))

(event `PlayerOrBotDied`
  (params (CurrentHealth :type "Object Object Reference") (CurrentShield :type "Object Object Reference") (HealthChange :type "Object Object Reference") (ShieldChange :type "Object Object Reference") (HitInfo :type "IGS_HitInfo Object Reference (by ref)")))

(event `DialogueStarted_E646BE0948CB57B3E0F0CE9BEE89CA41`
  (params (LineIndex :type Integer)))

(event `StartBlackscreenSound`)

(event `DialogueFinished_80BA75504AD858512EDC068FCB7C460B`
  (params (LineIndex :type Integer)))

(event `SetupSegment_3Stars`)

(event `DialogueStarted_BF4B34754166F7B85E4D4985665BA794`
  (params (LineIndex :type Integer)))

(event `CheckForSpecialTierRatioOnPhaseChanged`
  (params (inPressurePhase :type "EIGS_PressurePhase Enum" :default "PP_Unknown")))

(event `VO_SetReminder`
  (params (VO :type "Array of Object Object Reference (by ref)")))

(event `DialogueStarted_B5CE670B45EDF888D163B9A9D94FD0B8`
  (params (LineIndex :type Integer)))

(event `FinalDialoguePlayed`)

(event `StartBlackscreenDialogues`)

(event `OnAllDiedOrDowned`)

(event `SCMEvent_OnFinalDialogueDone`)

(event `SCM_Base_INIT_Setup`
  (params (inWaveManagerData :type "IGS_WaveManagerData Object Reference") (ActivateGeneralListener :type Boolean)))

(event `DialogueLineFinished_80BA75504AD858512EDC068FCB7C460B`
  (params (LineIndex :type Integer)))

(event `Private_OnPlayerOrBotRegistered`
  (params (inCharacter :type "IGS_GameCharacterFramework Object Reference")))

(event `DialogueStarted_564B97D3460CBFFC602F72A8EE34575F`
  (params (LineIndex :type Integer)))

(event `SCM_Base_BotsBlend`
  (params (BlendPointsGroup :type "IGS_WaypointFramework Object Reference")))

(event `DialogueLineStarted_E646BE0948CB57B3E0F0CE9BEE89CA41`
  (params (LineIndex :type Integer)))

(event `PlayBlackscreenStartSound`
  (params (AkEvent :type "AkAudioEvent Object Reference")))

(event `DialogueFinished_673F9B4F492ECD8C1AE5C1904D617B87`
  (params (LineIndex :type Integer)))

(event `Setup_SegmentByStars`)

(event `DialogueLineStarted_BF4B34754166F7B85E4D4985665BA794`
  (params (LineIndex :type Integer)))

(event `SetupMultiplayerSpecialTierSpawns`)

(event `Private_PlayReminderVO`)

(event `DialogueLineStarted_B5CE670B45EDF888D163B9A9D94FD0B8`
  (params (LineIndex :type Integer)))

(event `SCM_StartEndMission`)

(event `DialogueFinished_63FA7185485AA2D148C051BA43B0B306`
  (params (LineIndex :type Integer)))

(event `EndFading`)

(event `SCMEvent_OnBlascreenEndStarted`)

(event `SCM_Base_AfterAssaultBuildup`)

(event `DialogueFinished_447BA1524613421CE358B482FA6FBBB9`
  (params (LineIndex :type Integer)))

(event `SetupSegment_2Stars`)

(event `DialogueLineStarted_564B97D3460CBFFC602F72A8EE34575F`
  (params (LineIndex :type Integer)))

(event `SCM_Base_OnMatchStarted`)

(event `DialogueLineFinished_E646BE0948CB57B3E0F0CE9BEE89CA41`
  (params (LineIndex :type Integer)))

(event `OnCharacterRegisteredEvent_Event_0`
  (params (inCharacter :type "IGS_GameCharacterFramework Object Reference")))

(event `DialogueStarted_673F9B4F492ECD8C1AE5C1904D617B87`
  (params (LineIndex :type Integer)))

(event `Setup_DefaultStarsByHeat`)

(event `DialogueLineFinished_BF4B34754166F7B85E4D4985665BA794`
  (params (LineIndex :type Integer)))

(event `SCM_Base_MusicAndWaveManager_Curve`
  (params (AssaultBuildUp_START_IN :type "Object Object Reference")))

(event `VO_BossLastAlive`)

(event `DialogueLineFinished_B5CE670B45EDF888D163B9A9D94FD0B8`
  (params (LineIndex :type Integer)))

(event `SCM_FinishEndMissionNoResultScreen`)

(event `DialogueStarted_63FA7185485AA2D148C051BA43B0B306`
  (params (LineIndex :type Integer)))

(event `SetupBlackscreenFadeOut`)

(event `SCMEvent_OnAlarmStarted`)

(event `PlayersOrBotsHealthStateChanged`
  (params (HealthState :type "EIGS_HealthState Enum" :default "HS_Normal")))

(event `DialogueStarted_447BA1524613421CE358B482FA6FBBB9`
  (params (LineIndex :type Integer)))

(event `SetupSegment_1Star`)

(event `DialogueLineFinished_564B97D3460CBFFC602F72A8EE34575F`
  (params (LineIndex :type Integer)))

(event `SCM_Base_OnAlarmed`
  (params (AlarmReason :type "EIGS_AlarmReason Enum" :default "Alarm_UNKNOWN")))

(event `DialogueStarted_007EBB0340ADB5772A956A9D2C2A325C`
  (params (LineIndex :type Integer)))

(event `Debug_Swat_SpawningLeaving`)

(event `DialogueLineStarted_673F9B4F492ECD8C1AE5C1904D617B87`
  (params (LineIndex :type Integer)))

(event `SetupSegment_Increment`)

(event `Approach_110789DA42D5AE8606F227A148892C07`
  (params (Character :type "IGS_GameCharacterFramework Object Reference")))

(event `SpawnWaveManagerVehicles`)

(event `VO_BossInjured`)

(event `SCMEvent_OnBlackScreenFadeOut`)

(event `SCM_FinishEndMission`)

(event `DialogueLineStarted_63FA7185485AA2D148C051BA43B0B306`
  (params (LineIndex :type Integer)))

(event `StopBlackScreenDialogues`)

(event `SCMEvent_OnPlayerDowned`)

(event `AssembleScript_SmallHit`
  (params (ScenarioVariation :type Integer) (EnumByte :type Byte)))

(event `DialogueLineStarted_447BA1524613421CE358B482FA6FBBB9`
  (params (LineIndex :type Integer)))

(event `Setup_SCM_WaveManagerDefaults`
  (params (SpawnWaveManagerVehicles :type Boolean) (CustomStars :type Integer)))

(event `self.ReceiveBeginPlay`)

(event `DialogueLineStarted_007EBB0340ADB5772A956A9D2C2A325C`
  (params (LineIndex :type Integer)))

(event `OnCharacterUnregisteredEvent_Event_0`
  (params (inCharacter :type "IGS_GameCharacterFramework Object Reference") (inReason :type "EIGS_UnregisterReason Enum" :default "UR_EndPlay")))

(event `DialogueLineFinished_673F9B4F492ECD8C1AE5C1904D617B87`
  (params (LineIndex :type Integer)))

(event `SCM_Base_EndlessAssaultTriggered`)

(event `Arrive_110789DA42D5AE8606F227A148892C07`
  (params (Character :type "IGS_GameCharacterFramework Object Reference")))

(event `SetupSegment_5Stars`)

(event `OnLoaded_BA95395D4C1BA165DF4CD890B39FBC49`
  (params (Loaded :type "Object Object Reference")))

(event `SCMEvent_OnAllPlayersDead`)

(event `OnLoadedEvent`)

(event `DialogueLineFinished_63FA7185485AA2D148C051BA43B0B306`
  (params (LineIndex :type Integer)))

(fn `Get_SCA`
  (params (SCA_Tag :type "Object Object Reference"))
  (returns (SCA :type "IGS_ScriptActorBase Object Reference"))
  (return ""))

(fn `GetAllAlivePlayersAndBots`
  (returns (AllPlayersAndBots :type "Array of IGS_GameCharacterFramework Object Reference"))
  (locals (Local_AllAlivePlayersAndBots :type "Array of IGS_GameCharacterFramework Object Reference"))
  (return))

(fn `GetAllPlayersAndBots`
  (returns (AllPlayersAndBots :type "Array of IGS_GameCharacterFramework Object Reference"))
  (locals (Local_AllPlayersAndBots :type "Array of IGS_GameCharacterFramework Object Reference"))
  (return))

(fn `GetMissionResult`
  (returns (MissionResult :type "ECommonMissionResult Enum"))
  (return "Res_UNKNOWN"))

(fn `GetMusicPackFromMusicTag`
  (params (MusicTag :type "GameplayTag Object Reference"))
  (returns (MusicPack :type "AkStateValue Object Reference"))
  (locals (NewLocalVar_0 :type "GameplayTag Object Reference"))
  (return ""))

(fn `GetSpecialTierRatio`
  (params (inFPS :type "EIGS_FPSDifficulty Enum" :default "FD_Unknown") (inStormIntensity :type Integer))
  (returns (HasOverride :type Boolean) (NewRatio :type "Object Object Reference"))
  (locals (Local_MultiplayerConfig :type "META_QuickPlayData Object Reference"))
  (return false "0.0"))

(fn `Is Last Player Alive`
  (returns (LastAlive :type Boolean) (LastCharacter :type "IGS_GameCharacterFramework Object Reference"))
  (return false ""))

(fn `IsCharacterBoss`
  (params (Character :type "IGS_GameCharacterFramework Object Reference"))
  (returns (IsBoss :type Boolean))
  (return false))

(fn `SCM_Base_SpawnEscapeVan`
  (params (VehicleSpawner :type "IGS_VehicleSpawner Object Reference"))
  (returns (EscapeVan :type "IGS_VehicleBase Object Reference"))
  (return ""))

(fn `Select SWAT Amount Based On Tier`
  (params (`Normal Tier` :type Integer) (`Special Tier` :type Integer))
  (returns (`SWAT Amount` :type Integer))
  (return 0))

(fn `SetMissionResult`
  (params (inMissionResult :type "ECommonMissionResult Enum" :default "Res_UNKNOWN"))
  (return))

(fn `SetMusicPack`
  (returns (MusicPackFound :type Boolean) (MusicPack :type "AkStateValue Object Reference"))
  (locals (Local_FinalCollection :type "META_MusicScenarioPacksTableRow Object Reference") (Local_FoundMissionCollection :type Boolean) (Local_CurrentCollection :type "META_MusicScenarioPacksTableRow Object Reference") (Local_CollectionFound :type Boolean))
  (return false ""))

(fn `SetupNPCsFromMeta`
  (return))