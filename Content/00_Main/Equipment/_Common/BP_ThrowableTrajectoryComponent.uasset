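; Actor component, by its name, that previews the trajectory of thrown equipment.
; Setup functions take a throwable class and a low-throw input, alongside events to start, stop and toggle the prediction.
; A timer update event, a path prediction function, a too-close check and a Niagara value setter suggest a periodically refreshed effect-based arc.
; All graph bodies are empty here, so only the interface is defined.
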(event `BreakLoop`)

(event `self.OnShowPredictionChanged`
  (params (inShow :type Boolean) (inPredictedClass :type "IGS_ThrowableInventoryObject Class Reference")))

(event `self.ReceiveBeginPlay`)

(event `StartPrediction`)

(event `OnUpdateTimer`)

(event `StopPrediction`)

(fn `CheckIfTooClose`
  (return))

(fn `Init Throwable`
  (params (inClass :type "IGS_ThrowableInventoryObject Object Reference (by ref)"))
  (return))

(fn `InitComponent`
  (return))

(fn `PredictPathPrototypeWay`
  (returns (OutLocations :type "Array of Vector Object Reference") (outHitResult :type "HitResult Object Reference") (outSuccess :type Boolean))
  (locals (Locations :type "Array of Vector Object Reference"))
  (return _ "" false))

(fn `Reset Variables`
  (params (inThrowableClass :type "IGS_ThrowableInventoryObject Object Reference") (inLowThrow :type Boolean))
  (return))

(fn `SetNiagaraValues`
  (return))

(fn `SetThrowableClass`
  (params (ThrowableClass :type "IGS_ThrowableInventoryObject Object Reference"))
  (return))